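; Obstacle actor that reacts to contact from actors tagged Player by reducing its own DefaultHP variable.
; The Collider overlap event subtracts DamageHP and clamps the result between zero and MaxHP.
; It prints the remaining HP, or a DeathWidgetCall placeholder string at zero, without changing the overlapping actor.
; Despite the asset name, its graphs contain no rotation logic.
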(event OnComponentBeginOverlap(collider)
  (params (OverlappedComponent :type Primitive%20Component%20Object%20Reference) (OtherActor :type Actor%20Object%20Reference) (OtherComp :type Primitive%20Component%20Object%20Reference) (OtherBodyIndex :type Integer) (bFromSweep :type Boolean) (SweepResult :type Hit%20Result%20Structure%20%28by%20ref%29))
  (if (Actor|ActorHasTag OtherActor "Player")
    (bind _output_get (Variables|Default|SetDefaultHP (Math|Float|Clamp(Float) (- (Variables|Default|GetDefaultHP) (Variables|Default|GetDamageHP)) 0.0 (Variables|Default|GetMaxHP))))
    (if (<= (Variables|Default|GetDefaultHP) 0.0)
      (Development|PrintString "DeathWidgetCall")
      (else
        (Development|PrintString (Utilities|String|ToString(Float) _output_get))))))

(event EventBeginPlay)

(event Collision|EventActorBeginOverlap
  (params (OtherActor :type Actor%20Object%20Reference)))

(event EventTick
  (params (DeltaSeconds :type Float%20%28single-precision%29)))

(fn ConstructionScript)
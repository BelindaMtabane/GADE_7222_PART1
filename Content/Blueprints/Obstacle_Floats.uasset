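; Obstacle_Floats is an obstacle Blueprint that reacts to projectile hits on its box collider.
; On overlap, the DefaultFirearm tag selects a cast to BP_DefaultProjectile, while anything untagged is tried as BP_SecondFirearm.
; A successful cast calls the matching damage function on BPGunCompartment and destroys the projectile; a failed cast prints a debug string.
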(event OnComponentBeginOverlap(BoxCollider)
  (params (OverlappedComponent :type Primitive%20Component%20Object%20Reference) (OtherActor :type Actor%20Object%20Reference) (OtherComp :type Primitive%20Component%20Object%20Reference) (OtherBodyIndex :type Integer) (bFromSweep :type Boolean) (SweepResult :type Hit%20Result%20Structure%20%28by%20ref%29))
  (if (Actor|ActorHasTag OtherActor "DefaultFirearm")
    (bind _asbp_default_projectile (Utilities|Casting|CastToBP_DefaultProjectile OtherActor)
      (:then
        (Default|DamageDefaultFirearm (Variables|Default|GetBP_GunCompartment))
        (Actor|DestroyActor _asbp_default_projectile))
      (:CastFailed
        (Development|PrintString "NoDefaultFirearm")))
    (else
      (bind _asbp_second_firearm (Utilities|Casting|CastToBP_SecondFirearm OtherActor)
        (:then
          (Default|DamageSecondFirearm (Variables|Default|GetBP_GunCompartment))
          (Actor|DestroyActor _asbp_second_firearm))
        (:CastFailed
          (Development|PrintString "NoSecondFirearm"))))))

(event EventBeginPlay)

(event Collision|EventActorBeginOverlap
  (params (OtherActor :type Actor%20Object%20Reference)))

(event EventTick
  (params (DeltaSeconds :type Float%20%28single-precision%29)))

(fn ConstructionScript)
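; BP_GunCompartment is a damageable gun compartment with a clamped health pool and a separate damage function for the default and second firearms.
; Each function subtracts its own damage amount, and only the default firearm's version prints the remaining health.
; At zero health, both destroy the actor GetActorOfClass returns for Obstacle_Floats, rather than the compartment itself.
; The event graph is empty, so both functions rely on external callers.
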(event EventBeginPlay)

(event EventTick
  (params (DeltaSeconds :type Float%20%28single-precision%29)))

(fn DamageDefaultFirearm
  (bind _output_get (Variables|Default|SetCurrentHealth (Math|Float|Clamp(Float) (- (Variables|Default|GetCurrentHealth) (Variables|Default|GetDamageApplied1)) 0.0 (Variables|Default|GetMaxHealth))))
  (Development|PrintString (Utilities|String|ToString(Float) _output_get))
  (if (<= (Variables|Default|GetCurrentHealth) 0.0)
    (bind _returnvalue (Actor|GetActorOfClass "/Game/Blueprints/Obstacle_Floats.Obstacle_Floats_C"))
    (Actor|DestroyActor _returnvalue)))

(fn DamageSecondFirearm
  (Variables|Default|SetCurrentHealth (Math|Float|Clamp(Float) (- (Variables|Default|GetCurrentHealth) (Variables|Default|GetDamageApplied2)) 0.0 (Variables|Default|GetMaxHealth)))
  (if (<= (Variables|Default|GetCurrentHealth) 0.0)
    (bind _returnvalue (Actor|GetActorOfClass "/Game/Blueprints/Obstacle_Floats.Obstacle_Floats_C"))
    (Actor|DestroyActor _returnvalue)))
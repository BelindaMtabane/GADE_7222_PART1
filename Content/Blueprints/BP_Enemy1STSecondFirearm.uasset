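; BP_Enemy1STSecondFirearm is an enemy firearm hit Blueprint that records player kills in the game instance.
; Any SphereCollider overlap prints a debug string, then reads the player character's DefaultHP.
; At exactly zero HP it increments EN1TotalKillsPLY on BP_StatsInterface.
; It applies no damage, and the "Player" tag check's result is unused, so overlaps are not filtered.
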(event OnComponentBeginOverlap(SphereCollider)
  (params (OverlappedComponent :type Primitive%20Component%20Object%20Reference) (OtherActor :type Actor%20Object%20Reference) (OtherComp :type Primitive%20Component%20Object%20Reference) (OtherBodyIndex :type Integer) (bFromSweep :type Boolean) (SweepResult :type Hit%20Result%20Structure%20%28by%20ref%29))
  (Actor|ActorHasTag OtherActor "Player")
  (Development|PrintString "bulletATKplayer2ND" true true "(R=0.249709,G=1.000000,B=0.304858,A=1.000000)")
  (bind _asbp_player_character (Utilities|Casting|CastToBP_PlayerCharacter (Game|GetPlayerCharacter 0)))
  (if (== (Variables|/Game/FirstShooterCHAR/Blueprints/BP_PlayerCharacter.BP_PlayerCharacter_C|GetDefaultHP _asbp_player_character) 0.0)
    (bind _asbp_stats_interface (Utilities|Casting|CastToBP_StatsInterface (Game|GetGameInstance)))
    (Variables|/Game/Blueprints/BP_StatsInterface.BP_StatsInterface_C|SetEN1TotalKills_PLY _asbp_stats_interface (+ (Variables|/Game/Blueprints/BP_StatsInterface.BP_StatsInterface_C|GetEN1TotalKills_PLY _asbp_stats_interface) 1))))

(event EventBeginPlay)

(event Collision|EventActorBeginOverlap
  (params (OtherActor :type Actor%20Object%20Reference)))

(event EventTick
  (params (DeltaSeconds :type Float%20%28single-precision%29)))

(fn ConstructionScript)
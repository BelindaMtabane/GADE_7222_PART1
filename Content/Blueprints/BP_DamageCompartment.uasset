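; BP_DamageCompartment tracks a health value and applies damage to it from two firearms.
; DamageDefaultFirearm and DamageSecondFirearm each subtract their own damage amount from CurrentHealth, clamp it between zero and MaxHealth, then print the result.
; The event graph is empty, so both functions rely on external callers, and nothing here handles health reaching zero.
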(event EventBeginPlay)

(event EventTick
  (params (DeltaSeconds :type Float%20%28single-precision%29)))

(fn DamageDefaultFirearm
  (bind _output_get (Variables|Default|SetCurrentHealth (Math|Float|Clamp(Float) (- (Variables|Default|GetCurrentHealth) (Variables|Default|GetDamageApplied1)) 0.0 (Variables|Default|GetMaxHealth))))
  (Development|PrintString (Utilities|String|ToString(Float) _output_get)))

(fn DamageSecondFirearm
  (bind _output_get (Variables|Default|SetCurrentHealth (Math|Float|Clamp(Float) (- (Variables|Default|GetCurrentHealth) (Variables|Default|GetDamageApplied2)) 0.0 (Variables|Default|GetMaxHealth))))
  (if true
    (Development|PrintString (Utilities|String|ToString(Float) _output_get))))
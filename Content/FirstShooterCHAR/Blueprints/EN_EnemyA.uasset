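; Enemy pawn that chases the player character once it spots a pawn through its PawnSensing component.
; OnSeePawn sets SeePlayer and calls CatchPlayer, which issues an AI MoveTo toward player 0 without checking which pawn was seen.
; SetRandomDestinations is an unfinished wander fallback: its MoveTo has no inputs, and its branch is unreachable here because SeePlayer is set just before the only call.
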(event OnSeePawn(PawnSensing)
  (params (Pawn :type Pawn%20Object%20Reference))
  (Variables|Default|SetSee%20Player? true)
  (CallFunction|CatchPlayer))

(event Custom|CatchPlayer
  (if (Variables|Default|GetSee%20Player?)
    (AI|AIMoveTo self "0, 0, 0" (Game|GetPlayerCharacter 0) 5.0 false)
    (else
      (CallFunction|SetRandomDestinations))))

(event EventBeginPlay)

(event Collision|EventActorBeginOverlap
  (params (OtherActor :type Actor%20Object%20Reference)))

(event EventTick
  (params (DeltaSeconds :type Float%20%28single-precision%29)))

(event EventSetRandomDestinations
  (AI|AIMoveTo 0 "0, 0, 0" 0 5.0 false))

(fn ConstructionScript)
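; EN_EnemyB is a first-person shooter enemy character that patrols waypoints and shoots players spotted by PawnSensing, unless its health is low.
; CatchPlayer loops between AIMoveTo and firing, always spawning first-gun projectiles and adding second-gun shots when equipped.
; Tag-checked capsule overlaps handle ammo, health and gun pickups plus projectile damage, with automatic reload or default-gun fallback.
; Death teleports it to a random respawn point with restored health.
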(event OnComponentBeginOverlap(CapsuleComponent)
  (params (OverlappedComponent :type Primitive%20Component%20Object%20Reference) (OtherActor :type Actor%20Object%20Reference) (OtherComp :type Primitive%20Component%20Object%20Reference) (OtherBodyIndex :type Integer) (bFromSweep :type Boolean) (SweepResult :type Hit%20Result%20Structure%20%28by%20ref%29))
  ;[0.15 0.15 0.15 0.5] Collider
  (if (Actor|ActorHasTag OtherActor "Amm")
    (Development|PrintString "Ammunition logic")
    (CallFunction|AddAmm)
    (if (>= (Variables|Default|GetCurrentEnemyAmm) 6.0)
      (Development|PrintString "AmmunitionFull"))
    (Actor|DestroyActor OtherActor)
    (elif (Actor|ActorHasTag OtherActor "HealthEN")
      (if (< (Variables|Default|GetCurrentEnemyHP) 75.0)
        (CallFunction|Health))
      (elif (Actor|ActorHasTag OtherActor "SECfirearm")
        (Variables|Default|SetCurrentEnemyGun 2)
        (Actor|DestroyActor OtherActor)
        (CallFunction|SecondGunCalled)
        (CallFunction|ShootPlayerSecondGun)
        (elif (Actor|ActorHasTag OtherActor "DefaultFirearm")
          (Actor|DestroyActor OtherActor)
          (CallFunction|EnemyDamagedHealth1)
          (elif (Actor|ActorHasTag OtherActor "SecondFirearm")
            (Actor|DestroyActor OtherActor)
            (CallFunction|EnemyDamagedHealth2)))))))

(event OnSeePawn(PawnSensing)
  (params (Pawn :type Pawn%20Object%20Reference))
  ;[0.15 0.15 0.15 0.5] SensingPickups
  (if (Actor|ActorHasTag Pawn "Player")
    (if (< (Variables|Default|GetDefaultEnemyHP) 25.0)
      (Variables|Default|SetSee%20Player? false)
      (else
        (Variables|Default|SetSee%20Player? true)))
    (CallFunction|CatchPlayer)
    (else
      (Development|PrintString "not player"))))

(event Custom|CustomEvent
  (params (OverlappedComponent :type Primitive%20Component%20Object%20Reference) (OtherActor :type Actor%20Object%20Reference) (OtherComp :type Primitive%20Component%20Object%20Reference) (OtherBodyIndex :type Integer) (bFromSweep :type Boolean) (SweepResult :type Hit%20Result%20Structure%20%28by%20ref%29))
  ;[0.15 0.15 0.15 0.5] Health, bullets, second gun, ammunition Mechanic
  (if (Actor|ActorHasTag OtherActor "Amm")
    (Development|PrintString "Ammunition logic")
    (CallFunction|AddAmm)
    (if (>= (Variables|Default|GetCurrentEnemyAmm) 6.0)
      (Development|PrintString "AmmunitionFull"))
    (Actor|DestroyActor OtherActor)
    (elif (Actor|ActorHasTag OtherActor "HealthEN")
      (if (< (Variables|Default|GetCurrentEnemyHP) 75.0)
        (CallFunction|Health)
        (Actor|DestroyActor OtherActor)
        (Development|PrintString "Health needs to be called"))
      (elif (Actor|ActorHasTag OtherActor "SECfirearm")
        (Variables|Default|SetCurrentEnemyGun 2)
        (Actor|DestroyActor OtherActor)
        (CallFunction|SecondGunCalled)
        (elif (Actor|ActorHasTag OtherActor "DefaultFirearm")
          (Actor|DestroyActor OtherActor)
          (elif (Actor|ActorHasTag OtherActor "SecondFirearm")
            (Actor|DestroyActor OtherActor)))))))

(event Custom|CatchPlayer
  ;[0.15 0.15 0.15 0.5] Enemy Movement & Attack
  (if (== (Variables|Default|GetSee%20Player?) true)
    (if (== (Variables|Default|GetCurrentEnemyGun) 1)
      _
      (else
        (CallFunction|ShootPlayerSecondGun)))
    (Components|Movement|StopMovementImmediately (Variables|Character|GetCharacterMovement))
    (CallFunction|StopSprinting)
    (CallFunction|ShootPlayerFirstGun)
    (AI|AIMoveTo self "0, 0, 0" (Game|GetPlayerController 0) 5.0 false
      (:then
        _)
      (:OnSuccess
        _))
    (CallFunction|StopSprinting)
    (Utilities|FlowControl|Delay 2.0)
    (Variables|Default|SetSee%20Player? false)
    (CallFunction|CatchPlayer)
    (else
      (CallFunction|SetRandomDestinations))))

(event Custom|ShootPlayerSecondGun
  ;[0.15 0.15 0.15 0.5] ProjectileMechanicTWO
  (bind _output_get (Variables|Default|SetBulletInventory (Math|Float|Clamp(Float) (- (Variables|Default|GetBulletInventory) (Variables|Default|GetBulletsEnemyShot)) 0.0 (Variables|Default|GetMaxEnemyBullets))))
  (Development|PrintString (Utilities|String|ToString(Float) _output_get) true true "(R=1.000000,G=0.351345,B=0.000000,A=1.000000)")
  (if (== (Variables|Default|GetBulletInventory) 0.0)
    (if (== (Variables|Default|GetCurrentEnemyAmm) 0.0)
      (if (== (Variables|Default|GetCurrentEnemyGun) 2)
        _
        (else
          _))
      (Variables|Default|SetCurrentEnemyGun 1)
      (CallFunction|DefaultGunCalled)
      (else
        (CallFunction|ReloadGun)
        (CallFunction|ShootPlayerSecondGun)))
    (else
      (Game|SpawnActorfromClass "/Game/Blueprints/BP_Enemy1STSecondFirearm.BP_Enemy1STSecondFirearm_C" (Transformation|GetWorldTransform (Variables|Default|GetArrow2)) "AlwaysSpawn" "MultiplyWithRoot" 0 0))))

(event Custom|ShootPlayerFirstGun
  ;[0.15 0.15 0.15 0.5] ProjectileMechanicONE
  (Game|SpawnActorfromClass "/Game/Blueprints/BP_Enemy1STFirearm1.BP_Enemy1STFirearm1_C" (Transformation|GetWorldTransform (Variables|Default|GetArrow1)) "AlwaysSpawn" "MultiplyWithRoot" 0 0))

(event Custom|ReloadGun
  ;[0.15 0.15 0.15 0.5] Reload
  (CallFunction|MinusAmm)
  (if (>= (Variables|Default|GetCurrentEnemyAmm) 1.0)
    (Variables|Default|SetBulletInventory 12.0)
    (Development|PrintString "AmmunitionUsed" true true "(R=1.000000,G=0.432058,B=0.000000,A=1.000000)")
    (else
      (Variables|Default|SetCurrentEnemyGun 1)
      (CallFunction|DefaultGunCalled))))

(event EventBeginPlay
  ;[0.15 0.15 0.15 0.5] Start
  (if (not (> (Variables|Default|GetCurrentEnemyPath) 0))
    (CallFunction|CatchPlayer)))

(event EventSpawnPointersActors
  ;[0.15 0.15 0.15 0.5] SpawnEnemy
  (bind _outactors (Actor|GetAllActorsOfClass "/Game/Blueprints/BP_WaypointsRandom1.BP_WaypointsRandom1_C"))
  (bind _outitem (Utilities|Array|Random _outactors))
  (Transformation|SetActorLocation (Transformation|GetActorLocation _outitem) false false)
  (Variables|Default|SetDefaultEnemyHP 1e+02)
  (CallFunction|CatchPlayer))

(event EventEnemyDamagedHealth1
  ;[0.15 0.15 0.15 0.5] Health decrease one
  (bind _output_get (Variables|Default|SetDefaultEnemyHP (Math|Float|Clamp(Float) (- (Variables|Default|GetDefaultEnemyHP) (Variables|Default|GetDamageEnemyHP%201)) 0.0 (Variables|Default|GetMaxEnemyHP))))
  (if (<= (Variables|Default|GetDefaultEnemyHP) 0.0)
    (CallFunction|SpawnPointersActors)
    (else
      (Development|PrintString (Utilities|String|ToString(Float) _output_get)))))

(event EventEnemyDamagedHealth2
  ;[0.15 0.15 0.15 0.5] Health decrease two
  (bind _output_get (Variables|Default|SetDefaultEnemyHP (Math|Float|Clamp(Float) (- (Variables|Default|GetDefaultEnemyHP) (Variables|Default|GetDamageEnemyHP_2)) 0.0 (Variables|Default|GetMaxEnemyHP))))
  (if (<= (Variables|Default|GetDefaultEnemyHP) 0.0)
    (CallFunction|SpawnPointersActors)
    (else
      (Development|PrintString (Utilities|String|ToString(Float) _output_get)))))

(event EventSetRandomDestinations
  ;[0.15 0.15 0.15 0.5] Waypoints
  (AI|AIMoveTo self "0, 0, 0" (Utilities|Array|Get(acopy) (Variables|Default|GetEnemyWayPaths) (Variables|Default|GetCurrentEnemyPath)) 5.0 false
    (:OnSuccess
      (Math|Integer|IncrementInt (Variables|Default|GetCurrentEnemyPath)
        (:%20%20
          (if (>= (Variables|Default|GetCurrentEnemyPath) (Utilities|Array|Length (Variables|Default|GetEnemyWayPaths)))
            (Variables|Default|SetCurrentEnemyPath 0))
          (Utilities|FlowControl|Delay 1.2)
          (CallFunction|SetRandomDestinations))))))

(fn ConstructionScript)

(fn RightMovement
  (bind _returnvalue (Pawn|GetControlRotation :!class /Script/Engine.Pawn))
  (Pawn|Input|AddMovementInput (Math|Vector|GetRightVector (Math|Rotator|MakeRotator (.roll _returnvalue) 0.0 (.yaw _returnvalue))) (Variables|Default|GetAction%20Value%20X) false))

(fn ForwardMovement
  (bind _returnvalue (Pawn|GetControlRotation :!class /Script/Engine.Pawn))
  (Pawn|Input|AddMovementInput (Math|Vector|GetForwardVector (Math|Rotator|MakeRotator (.roll _returnvalue) 0.0 (.yaw _returnvalue))) (Variables|Default|GetAction%20Value%20Y) false))

(fn Sprinting
  (Variables|/Script/Engine.CharacterMovementComponent|SetMaxWalkSpeed (Variables|Character|GetCharacterMovement) (Variables|Default|GetRunEnemySpeed)))

(fn StopSprinting
  (Variables|/Script/Engine.CharacterMovementComponent|SetMaxWalkSpeed (Variables|Character|GetCharacterMovement) (Variables|Default|GetWalkEnemySpeed)))

(fn DefaultGunCalled
  (Rendering|SetVisibility (Variables|Default|GetDefaultGun) true false)
  (Rendering|SetVisibility (Variables|Default|GetSecondGun) false false)
  (Development|PrintString "DefaultGunCalled"))

(fn SecondGunCalled
  (Rendering|SetVisibility (Variables|Default|GetSecondGun) true false)
  (Rendering|SetVisibility (Variables|Default|GetDefaultGun) false false)
  (Development|PrintString "SecondGunCalled"))

(fn AddAmm
  (bind _output_get (Variables|Default|SetCurrentEnemyAmm (Math|Float|Clamp(Float) (+ (Variables|Default|GetCurrentEnemyAmm) (Variables|Default|GetAddEnemyAmm)) 0.0 (Variables|Default|GetFullEnemyAmm))))
  (Development|PrintString (Utilities|String|ToString(Float) _output_get)))

(fn MinusAmm
  (bind _output_get (Variables|Default|SetCurrentEnemyAmm (Math|Float|Clamp(Float) (- (Variables|Default|GetCurrentEnemyAmm) (Variables|Default|GetMinusEnemyAmm)) 0.0 (Variables|Default|GetFullEnemyAmm))))
  (Development|PrintString (Utilities|String|ToString(Float) _output_get) true true "(R=1.000000,G=0.000000,B=0.137026,A=1.000000)"))

(fn Health
  (bind _output_get (Variables|Default|SetDefaultEnemyHP (Math|Float|Clamp(Float) (+ (Variables|Default|GetDefaultEnemyHP) (Variables|Default|GetAddedEnemyHP)) 0.0 (Variables|Default|GetMaxEnemyHP))))
  (if (>= (Variables|Default|GetDefaultEnemyHP) 1e+02)
    (Development|PrintString "healthfull")
    (else
      (Development|PrintString (Utilities|String|ToString(Float) _output_get) true true "(R=0.000000,G=1.000000,B=0.056098,A=1.000000)"))))
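; BP_HealthEnergy2 is a health pickup placeholder that prints "HealthUP" and changes no health value.
; A Sphere overlap by a Player-tagged actor hides the sphere and three mesh surfaces, then after a delay reshows only the sphere and prints.
; The fallback enemy tag checks test the pickup's own tags instead of the overlapping actor's.
; Hiding affects visibility only, leaving collision untouched.
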(event OnComponentBeginOverlap(Sphere)
  (params (OverlappedComponent :type Primitive%20Component%20Object%20Reference) (OtherActor :type Actor%20Object%20Reference) (OtherComp :type Primitive%20Component%20Object%20Reference) (OtherBodyIndex :type Integer) (bFromSweep :type Boolean) (SweepResult :type Hit%20Result%20Structure%20%28by%20ref%29))
  (if (Actor|ActorHasTag OtherActor "Player")
    (Rendering|SetVisibility (Variables|Default|GetSphere) false false :!label _label)
    (Utilities|FlowControl|Delay 4.0)
    (Rendering|SetVisibility (Variables|Default|GetSphere) true false)
    (Development|PrintString "HealthUP" true true "(R=1.000000,G=0.536602,B=0.000000,A=1.000000)")
    (elif (Actor|ActorHasTag "EnemyA")
      (goto _label)
      (elif (Actor|ActorHasTag "EnemyB")
        (goto _label)
        (elif (Actor|ActorHasTag "EnemyC")
          (goto _label)
          (elif (Actor|ActorHasTag "EnemyD")
            (goto _label)))))))

(event EventBeginPlay)

(event Collision|EventActorBeginOverlap
  (params (OtherActor :type Actor%20Object%20Reference)))

(event EventTick
  (params (DeltaSeconds :type Float%20%28single-precision%29)))

(fn ConstructionScript)